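; Evil battery pickup that plays a hostile electric arc and explosion effect when collected.
; WasCollected attaches the arc to the pickup mesh and re-aims its beam at the player's left hand socket through a short Delay loop.
; A one-second Delay then spawns an explosion at that hand, plays a hurt sound at world origin and calls the parent WasCollected.
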(event `self.WasCollected`
  (bind _returnvalue (`SceneComponent.GetSocketLocation` (`Character.Mesh` (`GameplayStatics.GetPlayerCharacter` 0)) "LeftHandSocket"))
  (bind _returnvalue_2 (`GameplayStatics.SpawnEmitterAttached` "/Game/ExampleContent/Effects/ParticleSystems/P_electricity_arcEvil.P_electricity_arcEvil" (`self.PickupMesh`) "None" (0.0 0.0 0.0) (struct) (1.0 1.0 1.0) "SnapToTargetIncludingScale"))
  ;[1 1 1] Update beam target when character is running around
  (`ParticleSystemComponent.SetBeamTargetPoint` _returnvalue_2 0 _returnvalue 0 :!label _label)
  (`|ExecutionSequence`
    (:`then_0`
      (`KismetSystemLibrary.Delay` 1.0)
      (`GameplayStatics.SpawnEmitterAtLocation` "/Game/StarterContent/Particles/P_Explosion.P_Explosion" _returnvalue)
      (`GameplayStatics.PlaySoundAtLocation` "/Game/Sounds/FireHurt.FireHurt" (0.0 0.0 0.0) (struct) 1.0 1.0 0.0 null null null)
      (`parent.WasCollected`))
    (:`then_1`
      (`KismetSystemLibrary.Delay` 0.1)
      (goto _label))))

(fn `UserConstructionScript`)